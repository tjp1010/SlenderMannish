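; BP_Slendy is a Slender Man-style enemy that constantly stalks the player and ends the game on contact.
; Each Tick it turns SlendyMesh in yaw toward the player and slowly eases it toward an offset point near them.
; Movement interpolates the mesh component's world location without sweep or pathfinding.
; A capsule overlap with the player calls HandleGameOver(false) on BP_SlenderGamemode.
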(event `self.ReceiveTick`
  (params (DeltaSeconds :type "Float (single-precision)"))
  (`self.Rotate to Player` DeltaSeconds)
  (`self.MoveToPLayer` DeltaSeconds))

(event `self.Capsule.OnComponentBeginOverlap`
  (params (OverlappedComponent :type "PrimitiveComponent Object Reference") (OtherActor :type "Actor Object Reference") (OtherComp :type "PrimitiveComponent Object Reference") (OtherBodyIndex :type Integer) (bFromSweep :type Boolean) (SweepResult :type "HitResult Structure (by ref)"))
  (if (== OtherActor (`GameplayStatics.GetPlayerCharacter` 0))
    (bind _asbp_slender_gamemode (cast `/Game/MyContent/Gamemode/BP_SlenderGamemode` (`GameplayStatics.GetGameMode`)))
    (`/Game/MyContent/Gamemode/BP_SlenderGamemode.HandleGameOver` _asbp_slender_gamemode false)))

(fn `MoveToPLayer`
  (params (deltaTime :type "Float (double-precision)"))
  (`SceneComponent.K2_SetWorldLocation` (`self.SlendyMesh`) (`KismetMathLibrary.VInterpTo` (`SceneComponent.K2_GetComponentLocation` (`self.SlendyMesh`)) (`KismetMathLibrary.MakeVector` (+ (.x (`self.K2_GetActorLocation` (`GameplayStatics.GetPlayerCharacter` 0))) 50.0) (+ (.y (`self.K2_GetActorLocation` (`GameplayStatics.GetPlayerCharacter` 0))) 50.0) (- (.z (`self.K2_GetActorLocation` (`GameplayStatics.GetPlayerCharacter` 0))) 96.0)) deltaTime 0.2) false false))

(fn `Rotate to Player`
  (params (DeltaTime :type "Float (double-precision)"))
  (bind _returnvalue (`SceneComponent.K2_GetComponentRotation` (`self.SlendyMesh`)))
  ;[1 0 0] LookingAtPlayer
  (`SceneComponent.K2_SetWorldRotation` (`self.SlendyMesh`) (`KismetMathLibrary.RInterpTo` _returnvalue (`KismetMathLibrary.MakeRotator` (.roll _returnvalue) (.pitch _returnvalue) (- (.yaw (`KismetMathLibrary.FindLookAtRotation` (`SceneComponent.K2_GetComponentLocation` (`self.SlendyMesh`)) (`self.K2_GetActorLocation` (`GameplayStatics.GetPlayerCharacter` 0)))) 90.0)) DeltaTime 5.0) false false))

(fn `UserConstructionScript`)