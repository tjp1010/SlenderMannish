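; BP_MainHUD is an actor that manages the main game HUD and tracks note collection in a Slender-style game.
; On BeginPlay it creates the W_MainGameHud widget and adds it to the viewport.
; IncramentNotes raises the collected count, updates the counter text with a hardcoded "/8" total, then checks it against MaxNotes2Collect.
; When they match, it calls HandleGameOver(true) on BP_SlenderGamemode.
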(event `self.ReceiveBeginPlay`
  (bind _returnvalue (`|CreateWidget` "/Game/MyContent/Widgets/W_MainGameHud.W_MainGameHud_C"))
  (bind _output_get (set `self.Main Game Hud Ref` _returnvalue))
  (`UserWidget.AddToViewport` _output_get 0))

(fn `IncramentNotes`
  (bind _result (`/Engine/EditorBlueprintResources/StandardMacros.IncrementInt` (`self.NumbNotesCollected`))
    (:`  `
      (`TextBlock.SetText` (`/Game/MyContent/Widgets/W_MainGameHud.NumberCollected` (`self.Main Game Hud Ref`)) (`|FormatText` "{NumbNotesCollected}/8" _result))
      (`self.On All Notes Collected`))))

(fn `On All Notes Collected`
  (if (== (`self.NumbNotesCollected`) (`self.MaxNotes2Collect`))
    (bind _asbp_slender_gamemode (cast `/Game/MyContent/Gamemode/BP_SlenderGamemode` (`GameplayStatics.GetGameMode`)))
    (`/Game/MyContent/Gamemode/BP_SlenderGamemode.HandleGameOver` _asbp_slender_gamemode true)))

(fn `UserConstructionScript`)