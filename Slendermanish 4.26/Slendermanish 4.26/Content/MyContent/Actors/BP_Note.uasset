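; BP_Note is a collectible note actor that the player picks up with the Interact input.
; On BeginPlay it sets the prompt text on its W_Interact widget component and caches the player's BP_MainHUD.
; Collision overlap events track an Overlapped flag and toggle the prompt's visibility.
; Pressing Interact while overlapped increments the HUD's note count and destroys the actor, with no look-at check despite the graph comment.
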(event `self.ReceiveBeginPlay`
  (`|ExecutionSequence`
    (:`then_0`
      (bind _asw_interact (cast `/Game/MyContent/Widgets/W_Interact` (`WidgetComponent.GetUserWidgetObject` (`self.InteractWidget`))))
      (bind _output_get (set `self.As W Interact` _asw_interact))
      (set `/Game/MyContent/Widgets/W_Interact.TextToDisplay` (`self.InteractText`) _output_get))
    (:`then_1`
      (bind _asbp_main_hud (cast `/Game/MyContent/Gamemode/BP_MainHUD` (`PlayerController.GetHUD` (`GameplayStatics.GetPlayerController` 0))))
      (set `self.As BP Main HUD` _asbp_main_hud))))

(event `self.Collision.OnComponentBeginOverlap`
  (params (OverlappedComponent :type "PrimitiveComponent Object Reference") (OtherActor :type "Actor Object Reference") (OtherComp :type "PrimitiveComponent Object Reference") (OtherBodyIndex :type Integer) (bFromSweep :type Boolean) (SweepResult :type "HitResult Structure (by ref)"))
  ;[1 1 1] Toggle visibility of widget
  (set `self.Overlapped` true)
  (`SceneComponent.ToggleVisibility` (`self.InteractWidget`) false))

(event `self.Collision.OnComponentEndOverlap`
  (params (OverlappedComponent :type "PrimitiveComponent Object Reference") (OtherActor :type "Actor Object Reference") (OtherComp :type "PrimitiveComponent Object Reference") (OtherBodyIndex :type Integer))
  ;[1 1 1] Toggle visibility of widget
  (set `self.Overlapped` false)
  (`SceneComponent.ToggleVisibility` (`self.InteractWidget`) false))

(event `InputAction|Interact` :consume false
  (params (Key :type "Key Structure"))
  ;[1 1 1] If E pressed, destroy actor when looking at it
  (:`Pressed`
    (if (`self.Overlapped`)
      (`/Game/MyContent/Gamemode/BP_MainHUD.IncramentNotes` (`self.As BP Main HUD`))
      (`self.K2_DestroyActor`))))

(fn `UserConstructionScript`)